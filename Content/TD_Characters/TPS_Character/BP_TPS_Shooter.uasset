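; Third-person shooter character Blueprint that adds an aim-point HUD on BeginPlay and handles iron-sight aiming and rifle fire.
; Holding IA_Aim slows movement, turns the body with the controller and drives a timeline that shortens the camera boom and narrows FOV, reversing on release.
; IA_Shoot works only while aiming, playing a fire montage and rifle sound, with a DoOnce reset on montage completion to pace shots; no hit logic.
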(event Input|EnhancedActionEvents|EnhancedInputActionIA_Aim
  (params (ActionValue :type Boolean) (ElapsedSeconds :type Float%20%28double-precision%29) (TriggeredSeconds :type Float%20%28double-precision%29) (InputAction :type Input%20Action%20Object%20Reference :default "/Game/ThirdPerson/Input/Actions/IA_Aim.IA_Aim"))
  (bind _charactermovement (Variables|Character|GetCharacterMovement))
  (bind _charactermovement_2 (Variables|Character|GetCharacterMovement))
  (:Started
    (Variables|ActionState|SetIronSightsAiming? true)
    (Variables|/Script/Engine.CharacterMovementComponent|SetbOrientRotationToMovement _charactermovement_2 false)
    (Variables|/Script/Engine.CharacterMovementComponent|SetbUseControllerDesiredRotation _charactermovement_2 true)
    (Variables|/Script/Engine.CharacterMovementComponent|SetMaxWalkSpeed _charactermovement_2 2e+02)
    (bind _camera_arm_length_factor (Timeline|Timeline_Aiming Play)
      (:Update
        (Variables|/Script/Engine.SpringArmComponent|SetTargetArmLength (Variables|Default|GetCameraBoom) (Math|Float|Lerp 3e+02 5e+01 _camera_arm_length_factor))
        (Camera|SetFieldOfView (Variables|Default|GetFollowCamera) (Math|Float|Lerp 9e+01 45.0 _camera_arm_length_factor)))))
  (:Completed
    (Variables|ActionState|SetIronSightsAiming? false)
    (Variables|/Script/Engine.CharacterMovementComponent|SetbOrientRotationToMovement _charactermovement true)
    (Variables|/Script/Engine.CharacterMovementComponent|SetbUseControllerDesiredRotation _charactermovement false)
    (Variables|/Script/Engine.CharacterMovementComponent|SetMaxWalkSpeed _charactermovement (Variables|Default|GetDefaultMaxWalkSpeed))
    (Timeline|Timeline_Aiming ReverseFromEnd)))

(event Input|EnhancedActionEvents|EnhancedInputActionIA_Shoot
  (params (ActionValue :type Boolean) (ElapsedSeconds :type Float%20%28double-precision%29) (TriggeredSeconds :type Float%20%28double-precision%29) (InputAction :type Input%20Action%20Object%20Reference :default "/Game/ThirdPerson/Input/Actions/IA_Shoot.IA_Shoot"))
  (:Triggered
    (if (Variables|ActionState|GetIronSightsAiming?)
      (Utilities|FlowControl|DoOnce false :!label _label
        (:Completed
          (Animation|Montage|PlayMontage (Variables|Character|GetMesh) "/Game/TD_Characters/TPS_AnimationPack/AM_Fire_Rifle_Ironsights.AM_Fire_Rifle_Ironsights" 2.0
            (:then
              (Audio|PlaySoundatLocation "/Game/TD_Sound/S_AssaultRifleFire.S_AssaultRifleFire" (Transformation|GetWorldLocation (Variables|Default|GetSK_AR4)) "0, 0, 0" 5.0 1.0 0.0 0 0 0 0))
            (:OnCompleted
              (goto _label Reset))))))))

(event EventBeginPlay
  (bind _output_get (Variables|/Script/Engine.CharacterMovementComponent|SetMaxWalkSpeed (Variables|Character|GetCharacterMovement) 5e+02))
  (Variables|Default|SetDefaultMaxWalkSpeed _output_get)
  (bind _returnvalue (UserInterface|CreateWidget "/Game/TD_Characters/TPS_Character/WBP_HUD_AimPoint.WBP_HUD_AimPoint_C" (Game|GetPlayerController 0)))
  (UserInterface|Viewport|AddtoViewport _returnvalue 0))

(event Collision|EventActorBeginOverlap
  (params (OtherActor :type Actor%20Object%20Reference)))

(event EventTick
  (params (DeltaSeconds :type Float%20%28single-precision%29)))

(fn ConstructionScript)