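; BP_HoleWall is a destructible wall that paints bullet holes into its materials when it takes point damage.
; On BeginPlay it creates mask and diffuse render targets and feeds both to dynamic instances of the mesh materials.
; Each hit's collision UV positions two brush materials, drawn into those targets with shared random rotation and scale.
; A debug plane displays the mask target after each hit.
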(event Custom|CreateHoleEvent
  (bind _debugplane (Variables|Default|GetDebugPlane))
  (CallFunction|FuncCreateBulletHole (Utilities|Struct|MakeStruct_DestrutiveWall (.UV (Class|GameplayStatics|FindCollisionUV (Variables|Default|GetDamageHit))) "0.000000,0.000000,0.000000" "0.000000,0.000000,0.000000"))
  ;[1 1 1] Debug
  (bind _returnvalue (Rendering|Material|CreateDynamicMaterialInstance _debugplane 0 (Rendering|Material|GetMaterial _debugplane 0) "" :!class /Script/Engine.PrimitiveComponent))
  (Rendering|Material|SetTextureParameterValue _returnvalue "TEX" (Variables|Default|GetRenderTarget2D)))

(event Game|Damage|EventPointDamage
  (params (Damage :type Float%20%28single-precision%29) (DamageType :type Damage%20Type%20Object%20Reference) (HitLocation :type Vector :default "0, 0, 0") (HitNormal :type Vector :default "0, 0, 0") (HitComponent :type Primitive%20Component%20Object%20Reference) (BoneName :type Name :default "None") (ShotFromDirection :type Vector :default "0, 0, 0") (InstigatedBy :type Controller%20Object%20Reference) (DamageCauser :type Actor%20Object%20Reference) (HitInfo :type Hit%20Result%20Structure%20%28by%20ref%29))
  (Variables|Default|SetDamageHit HitInfo)
  (CallFunction|CreateHoleEvent))

(event EventBeginPlay
  (CallFunction|Init))

(fn ConstructionScript)

(fn Init
  (bind _materials (Variables|Default|GetMaterials))
  (Utilities|FlowControl|Sequence
    (:then_0
      ;[1 1 1] Create RenderTarget
      (bind _returnvalue (Rendering|CreateRenderTarget2D (Variables|Default|GetRTWidth) (Variables|Default|GetRTHeight) "RTF_RGBA8"))
      (Variables|Default|SetRenderTarget2D _returnvalue)
      (bind _returnvalue_2 (Rendering|CreateRenderTarget2D (Variables|Default|GetRTWidth) (Variables|Default|GetRTHeight) "RTF_RGBA8" "(R=0.000000,G=0.000000,B=0.000000,A=0.000000)"))
      (Variables|Default|SetDiffuseRenderTarget _returnvalue_2))
    (:then_1
      (if (> (Utilities|Array|Length _materials) 0)
        (for (_array_element _array_index) _materials
          (bind _returnvalue_3 (Rendering|Material|CreateDynamicMaterialInstance (Variables|Default|GetStaticMesh) _array_index _array_element "None" :!class /Script/Engine.PrimitiveComponent))
          ;[1 1 1] Set RT to dynamic material properties
          (Rendering|Material|SetTextureParameterValue _returnvalue_3 "DestructiveRT" (Variables|Default|GetRenderTarget2D))
          (Rendering|Material|SetTextureParameterValue _returnvalue_3 "DestructiveDiffuseRT" (Variables|Default|GetDiffuseRenderTarget)))
        ;[1 1 1] Create Brush material
        (bind _returnvalue_4 (Rendering|Material|CreateDynamicMaterialInstance "/Game/TD_Fracture/RT_Destructive/Mat_Brush.Mat_Brush" "None" "None" :!class /Script/Engine.KismetMaterialLibrary))
        (Variables|Default|SetBrushDMI _returnvalue_4)
        (bind _returnvalue_5 (Rendering|Material|CreateDynamicMaterialInstance "/Game/TD_Fracture/RT_Destructive/Mat_DiffuseBrush.Mat_DiffuseBrush" "None" "None" :!class /Script/Engine.KismetMaterialLibrary))
        (Variables|Default|SetDiffuseBrushDMI _returnvalue_5)
        (else
          (Development|PrintString "Destructive Material NULL" true true "(R=1.000000,G=0.000000,B=0.065193,A=1.000000)" 2e+01))))))

(fn FuncCreateBulletHole
  (params (HitData :type Struct%20Destrutive%20Wall%20Structure))
  (bind _uv (Utilities|Struct|BreakStruct_DestrutiveWall HitData))
  (bind _brushdmi (Variables|Default|GetBrushDMI))
  (bind _diffusebrushdmi (Variables|Default|GetDiffuseBrushDMI))
  (bind _diffusebrushdmi_2 (Variables|Default|GetDiffuseBrushDMI))
  (bind _masksizemax (Variables|Default|GetMaskSIzeMax))
  (bind _masksizemin (Variables|Default|GetMaskSizeMin))
  (bind _brushdmi_2 (Variables|Default|GetBrushDMI))
  (bind (_x _y) (Math|Vector2D|BreakVector2D _uv))
  (bind _returnvalue (Math|Random|RandomFloatinRange _masksizemin _masksizemax))
  (bind _linearcolor (Utilities|Struct|MakeLinearColor _x _y 0.0 0.0))
  (Utilities|FlowControl|Sequence
    (:then_0
      (Utilities|IsValid _brushdmi
        (:Is%20Valid
          (Rendering|Material|SetVectorParameterValue _brushdmi "Location" _linearcolor :!class /Script/Engine.MaterialInstanceDynamic)
          (bind _output_get (LocalVariables|SetTempRotation (Math|Random|RandomFloat)))
          (Rendering|Material|SetScalarParameterValue _brushdmi "Rotation" _output_get :!class /Script/Engine.MaterialInstanceDynamic)
          (Rendering|Material|SetTextureParameterValue _brushdmi_2 "TEX" (Variables|Default|GetMaskTex))
          (bind _output_get_2 (LocalVariables|SetTempSizes (Utilities|Struct|MakeLinearColor _returnvalue _returnvalue 0.0 0.0)))
          (Rendering|Material|SetVectorParameterValue _brushdmi_2 "DownScale" _output_get_2 :!class /Script/Engine.MaterialInstanceDynamic)
          (Rendering|DrawMaterialtoRenderTarget (Variables|Default|GetRenderTarget2D) (Variables|Default|GetBrushDMI))
          (Rendering|Material|SetVectorParameterValue _diffusebrushdmi "Location" _linearcolor :!class /Script/Engine.MaterialInstanceDynamic)
          (Rendering|Material|SetScalarParameterValue _diffusebrushdmi "Rotation" (LocalVariables|GetTempRotation) :!class /Script/Engine.MaterialInstanceDynamic)
          (Rendering|Material|SetTextureParameterValue _diffusebrushdmi_2 "TEX" (Variables|Default|GetBrushTex))
          (Rendering|Material|SetVectorParameterValue _diffusebrushdmi_2 "DownScale" (LocalVariables|GetTempSizes) :!class /Script/Engine.MaterialInstanceDynamic)
          (Rendering|DrawMaterialtoRenderTarget (Variables|Default|GetDiffuseRenderTarget) (Variables|Default|GetDiffuseBrushDMI)))))))