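; BP_TPS_Shooter is a third-person shooter character that spawns a rifle-socketed weapon and an aim-point HUD on begin play.
; Aiming switches to controller-facing rotation, slows movement and uses a timeline to pull in the camera boom and narrow FOV.
; Firing works only while aiming, with a DoOnce gated by montage completion setting the fire rate.
; Each shot traces from the camera, passes the result to the weapon and damages BP_Destructible hits.
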(event Input|EnhancedActionEvents|EnhancedInputActionIA_Aim
  (params (ActionValue :type Boolean) (ElapsedSeconds :type Float%20%28double-precision%29) (TriggeredSeconds :type Float%20%28double-precision%29) (InputAction :type Input%20Action%20Object%20Reference :default "/Game/ThirdPerson/Input/Actions/IA_Aim.IA_Aim"))
  (bind _charactermovement (Variables|Character|GetCharacterMovement))
  (bind _charactermovement_2 (Variables|Character|GetCharacterMovement))
  (:Started
    (Variables|ActionState|SetIronSightsAiming? true)
    (Variables|/Script/Engine.CharacterMovementComponent|SetbOrientRotationToMovement _charactermovement_2 false)
    (Variables|/Script/Engine.CharacterMovementComponent|SetbUseControllerDesiredRotation _charactermovement_2 true)
    (Variables|/Script/Engine.CharacterMovementComponent|SetMaxWalkSpeed _charactermovement_2 2e+02)
    (bind _camera_arm_length_factor (Timeline|Timeline_Aiming Play)
      (:Update
        (Variables|/Script/Engine.SpringArmComponent|SetTargetArmLength (Variables|Default|GetCameraBoom) (Math|Float|Lerp 3e+02 5e+01 _camera_arm_length_factor))
        (Camera|SetFieldOfView (Variables|Default|GetFollowCamera) (Math|Float|Lerp 9e+01 45.0 _camera_arm_length_factor)))))
  (:Completed
    (Variables|ActionState|SetIronSightsAiming? false)
    (Variables|/Script/Engine.CharacterMovementComponent|SetbOrientRotationToMovement _charactermovement true)
    (Variables|/Script/Engine.CharacterMovementComponent|SetbUseControllerDesiredRotation _charactermovement false)
    (Variables|/Script/Engine.CharacterMovementComponent|SetMaxWalkSpeed _charactermovement (Variables|Default|GetDefaultMaxWalkSpeed))
    (Timeline|Timeline_Aiming ReverseFromEnd)))

(event Input|EnhancedActionEvents|EnhancedInputActionIA_Shoot
  (params (ActionValue :type Boolean) (ElapsedSeconds :type Float%20%28double-precision%29) (TriggeredSeconds :type Float%20%28double-precision%29) (InputAction :type Input%20Action%20Object%20Reference :default "/Game/ThirdPerson/Input/Actions/IA_Shoot.IA_Shoot"))
  (bind _followcamera (Variables|Default|GetFollowCamera))
  (bind _returnvalue (Transformation|GetWorldLocation _followcamera))
  (:Triggered
    (if (Variables|ActionState|GetIronSightsAiming?)
      (Utilities|FlowControl|DoOnce false :!label _label
        (:Completed
          (Animation|Montage|PlayMontage (Variables|Character|GetMesh) "/Game/TD_Gameplay/TPS_AnimationPack/AM_Fire_Rifle_Ironsights.AM_Fire_Rifle_Ironsights" 2.0
            (:then
              (Audio|PlaySoundatLocation "/Game/TD_Sound/S_AssaultRifleFire.S_AssaultRifleFire" (Transformation|GetWorldLocation (Variables|/Script/Engine.Actor|GetRootComponent (Variables|Weapon|GetCurrentWeapon))) "0, 0, 0" 5.0 1.0 0.0 0 0 0 0)
              (bind (_outhit _returnvalue_2) (Collision|LineTraceByChannel _returnvalue (+ _returnvalue (* (Math|Vector|GetForwardVector _followcamera) 1e+04)) "TraceTypeQuery1" false 0 "None"))
              (Default|WeaponFire (Variables|Weapon|GetCurrentWeapon) (.HitActor (Collision|BreakHitResult _outhit)) (.TraceEnd (Collision|BreakHitResult _outhit)) (.Location (Collision|BreakHitResult _outhit)))
              (if _returnvalue_2
                (bind _asbp_destructible (Utilities|Casting|CastToBP_Destructible (.HitActor (Collision|BreakHitResult _outhit))))
                (Game|Damage|ApplyDamage _asbp_destructible 1e+01 (Pawn|GetController) self)))
            (:OnCompleted
              (goto _label Reset))))))))

(event EventBeginPlay
  (bind _returnvalue (Game|GetPlayerCameraManager 0))
  (bind _output_get (Variables|/Script/Engine.CharacterMovementComponent|SetMaxWalkSpeed (Variables|Character|GetCharacterMovement) 5e+02))
  (Variables|Default|SetDefaultMaxWalkSpeed _output_get)
  (bind _returnvalue_2 (UserInterface|CreateWidget "/Game/TD_Gameplay/TPS_Character/WBP_HUD_AimPoint.WBP_HUD_AimPoint_C" (Game|GetPlayerController 0)))
  (UserInterface|Viewport|AddtoViewport _returnvalue_2 0)
  (CallFunction|EquipWeapon)
  (Variables|/Script/Engine.PlayerCameraManager|SetViewPitchMin _returnvalue -6e+01)
  (Variables|/Script/Engine.PlayerCameraManager|SetViewPitchMax _returnvalue 6e+01))

(event Collision|EventActorBeginOverlap
  (params (OtherActor :type Actor%20Object%20Reference)))

(event EventTick
  (params (DeltaSeconds :type Float%20%28single-precision%29)))

(fn ConstructionScript)

(fn EquipWeapon
  (bind _returnvalue (Game|SpawnActorfromClass "/Game/TD_Gameplay/TPS_Weapon/BP_TPS_WeaponBase.BP_TPS_WeaponBase_C" (Math|Transform|MakeTransform (Transformation|GetActorLocation)) "Undefined" "MultiplyWithRoot" 0 0.0 0))
  (Utilities|IsValid _returnvalue
    (:Is%20Valid
      (Variables|Weapon|SetCurrentWeapon _returnvalue)
      (Transformation|AttachComponentToComponent _returnvalue (Variables|Character|GetMesh) "Socket_RightHandRifle" "SnapToTarget" "SnapToTarget" "KeepRelative" true))))