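; BP_TPS_WeaponBase is the base weapon for third-person shooting, providing a WeaponFire function that spawns the firing effects.
; WeaponFire spawns a gunfire GE and a tracer bullet GE at the muzzle socket.
; A camera trace along the supplied forward vector pre-aims the tracer at the hit or trace end, correcting camera-to-muzzle misalignment.
; The HitActor validity check has no follow-up, and no damage is applied here.
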(event EventBeginPlay)

(event Collision|EventActorBeginOverlap
  (params (OtherActor :type Actor%20Object%20Reference)))

(event EventTick
  (params (DeltaSeconds :type Float%20%28single-precision%29)))

(fn ConstructionScript)

(fn WeaponFire
  (params (HitActor :type Actor%20Object%20Reference) (ForwardVector :type Vector))
  (bind _weaponmesh (Variables|Default|GetWeaponMesh))
  (bind _returnvalue (Transformation|GetSocketLocation _weaponmesh "b_gun_muzzleflash"))
  (Utilities|FlowControl|Sequence
    (:then_0
      ;[1 0.5593 0] Muzzle
      (CallFunction|SpawnGE "/Game/TD_Gameplay/FX/Weapon_MuzzleFlash/GE_Weapon_GunFire.GE_Weapon_GunFire_C" (Math|Transform|MakeTransform (Transformation|GetSocketLocation (Variables|Default|GetWeaponMesh) "b_gun_muzzleflash") "0, 0, 0" "1.000000,1.000000,1.000000") false false 0 5.0)
      (Utilities|IsValid HitActor))
    (:then_1
      ;[0 0 0] 处理镜头方向与枪口方向的不一致性，通过镜头single trace预瞄准实现
      (bind _output_get (LocalVariables|SetCameraLocation (Camera|GetCameraLocation (Variables|/Script/Engine.PlayerController|GetPlayerCameraManager (Game|GetPlayerController 0)))))
      (bind (_outhit _returnvalue_2) (Collision|LineTraceByChannel _output_get (+ _output_get (* ForwardVector 1e+04)) "TraceTypeQuery1" false 0 "None"))
      (if _returnvalue_2
        (LocalVariables|SetTargetLocation (.Location (Collision|BreakHitResult _outhit)))
        (else
          (LocalVariables|SetTargetLocation (.TraceEnd (Collision|BreakHitResult _outhit)))))
      (CallFunction|SpawnGE "/Game/TD_Gameplay/FX/Weapon_TracerBullet/GE_Weapon_TracerBullet.GE_Weapon_TracerBullet_C" (Math|Transform|MakeTransform _returnvalue (Math|Rotator|FindLookatRotation _returnvalue (LocalVariables|GetTargetLocation)) "1.000000,1.000000,1.000000") false false 0 5.0))))