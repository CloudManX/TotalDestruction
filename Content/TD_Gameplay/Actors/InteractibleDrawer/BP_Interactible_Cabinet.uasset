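; BP_Interactible_Cabinet is an interactible cabinet whose physics-constrained drawer moves when hit.
; The construction script shifts Drawer01 vertically by a random multiple of a fixed step.
; BeginPlay sets the PhysicsConstraint reference position for its first frame.
; HitInteract applies a random-strength impulse along the actor's forward vector to the drawer and prints a debug greeting.
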(event EventBeginPlay
  (Class|PhysicsConstraintComponent|SetConstraintReferencePosition (Variables|Default|GetPhysicsConstraint) "Frame1" (Math|Vector|MakeVector 0.0 0.0 0.0)))

(event Collision|EventActorBeginOverlap
  (params (OtherActor :type Actor%20Object%20Reference)))

(event EventTick
  (params (DeltaSeconds :type Float%20%28single-precision%29)))

(event EventHitInteract
  (Physics|AddImpulse (Variables|Default|GetDrawer01) (* (Transformation|GetActorForwardVector) (Math|Random|RandomFloatinRange 1e+03 5e+03)) "None" false)
  (Development|PrintText "Hello"))

(fn ConstructionScript
  (Transformation|AddLocalOffset (Variables|Default|GetDrawer01) (Math|Vector|MakeVector 0.0 0.0 (* (Math|Random|RandomIntegerinRange 0 3) 32.0)) false false))